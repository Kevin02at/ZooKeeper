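; MoneySystem is an actor Blueprint for a duck-based money economy, creating the MoneyWidget and WP_ShopMenu widgets on BeginPlay.
; AddMoney, while DuckAmount is below two, derives a randomized visitor count from ducks and overwrites the shop menu's money with a multiple of it.
; The shop menu cast, starting-money setup and looping AddMoney timer are disconnected, so nothing here schedules income or supplies that menu reference.
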(event Custom|AddMoney
  (if (< (Variables|/Game/UI/WP_ShopMenu.WP_ShopMenu_C|GetDuckAmount (stale _aswp_shop_menu)) 2.0)
    (Variables|/Game/UI/WP_ShopMenu.WP_ShopMenu_C|SetVisitorAmount (stale _aswp_shop_menu) (+ (* (Variables|/Game/UI/WP_ShopMenu.WP_ShopMenu_C|GetDuckAmount (stale _aswp_shop_menu)) 2.0) (Math|Random|RandomFloatinRange 0.0 1e+01)))
    (Variables|/Game/UI/WP_ShopMenu.WP_ShopMenu_C|SetMoneyAmount (stale _aswp_shop_menu) (* (Variables|/Game/UI/WP_ShopMenu.WP_ShopMenu_C|GetVisitorAmount (stale _aswp_shop_menu)) 1e+01))
    (elif true
      _)))

(event EventBeginPlay
  (UserInterface|CreateWidget "/Game/Blueprints/MoneyWidget.MoneyWidget_C")
  (UserInterface|CreateWidget "/Game/UI/WP_ShopMenu.WP_ShopMenu_C"))

(event Collision|EventActorBeginOverlap
  (params (OtherActor :type Actor%20Object%20Reference)))

(event EventTick
  (params (DeltaSeconds :type Float%20%28single-precision%29)))

(fn ConstructionScript)