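; BP_Dummy is an AI pawn that follows the player and takes damage through a health value commented as hunger.
; Any damage adds to Health while it is below a fixed cap; after that, hits spawn a one-second spark effect instead.
; Pawn sensing sets a never-cleared seen flag and triggers AIMoveTo toward player zero.
; Tick turns the health bar widget toward the camera.
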(event `self.ReceiveAnyDamage`
  (params (Damage :type "Float (single-precision)") (DamageType :type "DamageType Object Reference") (InstigatedBy :type "Controller Object Reference") (DamageCauser :type "Actor Object Reference"))
  (bind _health (`self.Health`))
  ;[1 1 1] Health (Hunger) System
  (if (> 9.5 _health)
    (set `self.Health` (+ _health Damage))
    (`KismetSystemLibrary.PrintString` "Damage received")
    (else
      (bind _returnvalue (`GameplayStatics.SpawnEmitterAtLocation` "/Game/StarterContent/Particles/P_Sparks.P_Sparks" (`self.K2_GetActorLocation`)))
      (`KismetSystemLibrary.Delay` 1.0)
      (`ActorComponent.K2_DestroyComponent` _returnvalue))))

(event `self.PawnSensing.OnSeePawn`
  (params (Pawn :type "Pawn Object Reference"))
  ;[1 1 1] Follow Player
  (set `self.IsSeeingPlayer` true)
  (`self.FollowPlayer`))

(event `FollowPlayer`
  ;[1 1 1] Follow Player
  (if (`self.IsSeeingPlayer`)
    (`|AIMoveTo` self (0.0 0.0 0.0) (`GameplayStatics.GetPlayerCharacter` 0))))

(event `self.ReceiveTick`
  (params (DeltaSeconds :type "Float (single-precision)"))
  ;[1 1 1] Rotate widget (Health Bar) to face player
  (`SceneComponent.K2_SetWorldRotation` (`self.Widget`) (`KismetMathLibrary.FindLookAtRotation` (`SceneComponent.K2_GetComponentLocation` (`self.Widget`)) (`SceneComponent.K2_GetComponentLocation` (`PlayerCameraManager.TransformComponent` (`GameplayStatics.GetPlayerCameraManager` 0)))) false false))

(fn `UserConstructionScript`)